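; Stage light actor for the LoverHouse area that switches a rect light between six preset colors over time.
; After a fixed delay from BeginPlay, it plays a timeline whose floored ColorIndex track selects the color on each update.
; Each branch also stores the following index in CurrentColorIndex, which this graph never reads.
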(event EventBeginPlay
  (Utilities|FlowControl|Delay 33.0)
  (bind _colorindex (Timeline|Timeline Play)
    (:Update
      (switch int (Math|Float|Floor _colorindex)
        (:0
          (Rendering|Components|Light|SetLightColor (Variables|Default|GetRectLightComponent) "(R=0.514918,G=0.386430,B=0.552012,A=1.000000)" true)
          (Variables|Default|SetCurrentColorIndex 1))
        (:1
          (Rendering|Components|Light|SetLightColor (Variables|Default|GetRectLightComponent) "(R=0.806952,G=0.552012,B=0.278894,A=1.000000)" true)
          (Variables|Default|SetCurrentColorIndex 2))
        (:2
          (Rendering|Components|Light|SetLightColor (Variables|Default|GetRectLightComponent) "(R=0.822786,G=0.456411,B=0.603828,A=1.000000)" true)
          (Variables|Default|SetCurrentColorIndex 3))
        (:3
          (Rendering|Components|Light|SetLightColor (Variables|Default|GetRectLightComponent) "(R=0.152926,G=0.074214,B=0.061246,A=1.000000)" true)
          (Variables|Default|SetCurrentColorIndex 4))
        (:4
          (Rendering|Components|Light|SetLightColor (Variables|Default|GetRectLightComponent) "(R=0.508881,G=0.623961,B=0.473532,A=1.000000)" true)
          (Variables|Default|SetCurrentColorIndex 5))
        (:5
          (Rendering|Components|Light|SetLightColor (Variables|Default|GetRectLightComponent) "(R=0.539480,G=0.760525,B=0.904661,A=1.000000)" true)
          (Variables|Default|SetCurrentColorIndex 0))))))

(event EventTick
  (params (DeltaSeconds :type Float%20%28single-precision%29)))

(fn ConstructionScript)